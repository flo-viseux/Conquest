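; PC_MainMenu is a player controller that chooses between the main menu and the player HUD based on the current level.
; On BeginPlay, the local controller waits briefly, then checks the level name.
; The "Main" level triggers a custom event that adds W_PlayerHUD to the player screen, while any other level adds W_MainMenu to the viewport.
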(event Custom|Open%20player%20Widget
  (bind _returnvalue (UserInterface|CreateWidget "/Game/Blueprints/Player/W_PlayerHUD.W_PlayerHUD_C" self))
  (UserInterface|Viewport|AddtoPlayerScreen _returnvalue))

(event EventBeginPlay
  (if (Pawn|IsLocalController)
    (Utilities|FlowControl|Delay 1.0)
    (bind _returnvalue (Game|GetCurrentLevelName true))
    (if (Utilities|Enum|Equal(Enum) _returnvalue "Main")
      (CallFunction|OpenPlayerWidget)
      (else
        (bind _returnvalue_2 (UserInterface|CreateWidget "/Game/MainMenu/W_MainMenu.W_MainMenu_C" self))
        (UserInterface|Viewport|AddtoViewport _returnvalue_2 0)))))

(fn ConstructionScript)