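; BP_HandCards manages the player's hand of cards, tracking card actors in a CardsInHand array.
; AddCard spawns a BP_CCardActor, attaches it to PivotHandCards, stores it and calls PositionCards.
; PositionCards computes sine/cosine arc offsets per index, but applies them to the shared pivot rather than each card.
; RemoveCardFromHand only drops a card from the array, without destroying or repositioning.
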(fn ConstructionScript)

(fn AddCard
  (bind _returnvalue (Game|SpawnActorfromClass "/Game/Blueprints/Cards/BP_CCardActor.BP_CCardActor_C" (Math|Transform|MakeTransform "0, 0, 0") "Undefined" "MultiplyWithRoot" 0 0))
  (Transformation|AttachComponentToComponent _returnvalue (Variables|Default|GetPivotHandCards) "None" "KeepRelative" "KeepRelative" "KeepRelative" true)
  (Utilities|Array|Add (Variables|Default|GetCardsInHand) _returnvalue)
  (Development|PrintString (Utilities|String|ToString(Integer) (Utilities|Array|Length (Variables|Default|GetCardsInHand))))
  (CallFunction|PositionCards))

(fn PositionCards
  (Development|PrintString "here")
  (for (_ _array_index) (Variables|Default|GetCardsInHand)
    (Transformation|SetRelativeLocation (Variables|Default|GetPivotHandCards) (Math|Vector|MakeVector 0.0 (* (Math|Trig|Sin(Radians) (* _array_index 0.1)) 5e+01) (* (Math|Trig|Cos(Radians) (* _array_index 0.1)) 5e+01)) false false)))

(fn RemoveCardfromHand
  (params (Card :type BP%20C%20Card%20Actor%20Object%20Reference))
  (bind _cardsinhand (Variables|Default|GetCardsInHand))
  (if (Utilities|Array|ContainsItem _cardsinhand Card)
    (Utilities|Array|RemoveItem _cardsinhand Card)))