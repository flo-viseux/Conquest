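; BP_CCardActor is a card actor that displays a player-specific texture on its Cube mesh.
; SetCCardInfo looks up a DT_CCardInfo row and stores it as CardInfo with the given player index.
; A dynamic M_CardTexture material shows that player's texture, or T_Burst_M with a debug print for index -1.
; BeginPlay records the actor's location as CellPosition and applies the player texture after a short delay.
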(event Custom|Set%20CCardInfo
  (params (PlayerId :type Integer) (RowName :type Name))
  (bind _cardinfo (Variables|Default|GetCardInfo))
  (bind _returnvalue (Utilities|GetDataTableRow "/Game/Blueprints/Cards/DT_CCardInfo.DT_CCardInfo" RowName)
    (:then
      (Class|CCardActor|SetCardInfo (Utilities|Struct|MakeCCardInfo (.cardname _returnvalue) (.cardtype _returnvalue) PlayerId (.texture1 _returnvalue) (.texture2 _returnvalue) (.links _returnvalue)))
      (bind _returnvalue_2 (Rendering|Material|CreateDynamicMaterialInstance (Variables|Default|GetCube) 0 "/Game/Blueprints/Cards/M_CardTexture.M_CardTexture" "None" :!class /Script/Engine.PrimitiveComponent))
      (if (== (.playerindex _cardinfo) -1)
        (Development|PrintString "Hello")
        (Rendering|Material|SetTextureParameterValue _returnvalue_2 "Texture" "/Game/StarterContent/Textures/T_Burst_M.T_Burst_M")
        (else
          (Rendering|Material|SetTextureParameterValue _returnvalue_2 "Texture" (Utilities|Select :Index (.playerindex _cardinfo) :Option%200 (.texture1 _cardinfo) :Option%201 (.texture2 _cardinfo))))))))

(event EventBeginPlay
  (bind _cardinfo (Variables|Default|GetCardInfo))
  (Variables|Default|SetCellPosition (Transformation|GetActorLocation))
  (Utilities|FlowControl|Delay 0.2)
  (bind _returnvalue (Rendering|Material|CreateDynamicMaterialInstance (Variables|Default|GetCube) 0 "/Game/Blueprints/Cards/M_CardTexture.M_CardTexture" "None" :!class /Script/Engine.PrimitiveComponent))
  (Rendering|Material|SetTextureParameterValue _returnvalue "Texture" (Utilities|Select :Index (.playerindex _cardinfo) :Option%200 (.texture1 _cardinfo) :Option%201 (.texture2 _cardinfo))))

(fn ConstructionScript)