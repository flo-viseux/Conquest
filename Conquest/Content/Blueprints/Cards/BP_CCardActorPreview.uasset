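; BP_CCardActorPreview is a preview actor for a card, showing its texture and whether its placement is valid.
; On begin play it stores its location, then after a short delay creates a dynamic material and applies the owning player's texture.
; SetCCardInfo loads card data from DT_CCardInfo and updates that texture, using a burst texture when no player is set.
; Valid and invalid placement events tint the material white or red.
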(event Custom|Set%20CCardInfo
  (params (PlayerId :type Integer) (RowName :type Name))
  (bind _cardinfo (Variables|Default|GetCardInfo))
  (bind _returnvalue (Utilities|GetDataTableRow "/Game/Blueprints/Cards/DT_CCardInfo.DT_CCardInfo" RowName)
    (:then
      (Class|CCardActor|SetCardInfo (Utilities|Struct|MakeCCardInfo (.cardname _returnvalue) (.cardtype _returnvalue) PlayerId (.texture1 _returnvalue) (.texture2 _returnvalue) (.links _returnvalue)))
      (if (== (.playerindex _cardinfo) -1)
        (Rendering|Material|SetTextureParameterValue (Variables|Default|GetDynamic%20Mat%20Instance) "Texture" "/Game/StarterContent/Textures/T_Burst_M.T_Burst_M")
        (else
          (Rendering|Material|SetTextureParameterValue (Variables|Default|GetDynamic%20Mat%20Instance) "Texture" (Utilities|Select :Index (.playerindex _cardinfo) :Option%200 (.texture1 _cardinfo) :Option%201 (.texture2 _cardinfo))))))))

(event Custom|ValidPlacement
  (Rendering|Material|SetVectorParameterValue (Variables|Default|GetDynamic%20Mat%20Instance) "Color" "(R=1.000000,G=1.000000,B=1.000000,A=1.000000)" :!class /Script/Engine.MaterialInstanceDynamic))

(event Custom|UnvalidPlacement
  (Development|PrintString "Unvalid")
  (Rendering|Material|SetVectorParameterValue (Variables|Default|GetDynamic%20Mat%20Instance) "Color" "(R=1.000000,G=0.000000,B=0.000000,A=1.000000)" :!class /Script/Engine.MaterialInstanceDynamic))

(event EventBeginPlay
  (bind _cardinfo (Variables|Default|GetCardInfo))
  (Variables|Default|SetCellPosition (Transformation|GetActorLocation))
  (Utilities|FlowControl|Delay 0.2)
  (bind _returnvalue (Rendering|Material|CreateDynamicMaterialInstance (Variables|Default|GetCube) 0 "/Game/Blueprints/Cards/M_PreviewCardTexture.M_PreviewCardTexture" "None" :!class /Script/Engine.PrimitiveComponent))
  (bind _output_get (Variables|Default|SetDynamic%20Mat%20Instance _returnvalue))
  (Rendering|Material|SetTextureParameterValue _output_get "Texture" (Utilities|Select :Index (.playerindex _cardinfo) :Option%200 (.texture1 _cardinfo) :Option%201 (.texture2 _cardinfo))))

(fn ConstructionScript)