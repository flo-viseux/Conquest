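; Game mode for a two-player, turn-based card board game, handling match setup, hands, placement and turns.
; Once two players log in, it waits briefly, resets player states, deals three cards each from per-player decks and starts the game.
; Placed cards are built from data table rows, validated and followed by path checks.
; Turn-end events refill hands and pass turns through game and player states; Joker use decrements that player's count.
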(event Custom|Place%20Card%20On%20Board
  (params (NewCardLocation :type Vector) (CardDataRowName :type Name) (PlayerId :type Integer))
  ;[0 0 0] Place Card On Board
  (bind _returnvalue (Utilities|GetDataTableRow "/Game/Blueprints/Cards/DT_CCardInfo.DT_CCardInfo" CardDataRowName)
    (:then
      (bind _returnvalue_2 (Class|CGameModeBase|IsValidCardPlacement NewCardLocation (Utilities|Struct|MakeCCardInfo (.cardname _returnvalue) (.cardtype _returnvalue) PlayerId (.texture1 _returnvalue) (.texture2 _returnvalue) (.links _returnvalue))))
      (Class|CGameModeBase|PlaceCard NewCardLocation (Utilities|Struct|MakeCCardInfo (.cardname _returnvalue) (.cardtype _returnvalue) PlayerId (.texture1 _returnvalue) (.texture2 _returnvalue) (.links _returnvalue)))
      (if _returnvalue_2
        (Class|CGameModeBase|CheckGamePaths)
        (bind _asbp_cplayer_state (Utilities|Casting|CastToBP_CPlayerState (Game|GetPlayerState PlayerId)))
        (Variables|/Game/Blueprints/PlayerState/BP_CPlayerState.BP_CPlayerState_C|SetPlayerCardCount _asbp_cplayer_state (- (Variables|/Game/Blueprints/PlayerState/BP_CPlayerState.BP_CPlayerState_C|GetPlayerCardCount _asbp_cplayer_state) 1))
        (Default|CardPlaced _asbp_cplayer_state CardDataRowName)
        (Variables|/Game/Blueprints/PlayerState/BP_CPlayerState.BP_CPlayerState_C|SetCardPlacedCount _asbp_cplayer_state (+ (Variables|/Game/Blueprints/PlayerState/BP_CPlayerState.BP_CPlayerState_C|GetCardPlacedCount _asbp_cplayer_state) 1))))))

(event Custom|Add%20Card%20To%20Deck
  (params (PlayerID :type Integer))
  (bind _player1deckindex (Variables|Default|GetPlayer1DeckIndex))
  (bind _player2deckindex (Variables|Default|GetPlayer2DeckIndex))
  (bind _player2deck (Variables|Default|GetPlayer2Deck))
  (bind _player1deck (Variables|Default|GetPlayer1Deck))
  (bind _returnvalue (Utilities|Select :Index PlayerID :Option%200 _player1deck :Option%201 _player2deck))
  (bind _returnvalue_2 (Utilities|Select :Index PlayerID :Option%200 _player1deckindex :Option%201 _player2deckindex))
  ;[0 0 0] Add Card
  (bind _asbp_cplayer_state (Utilities|Casting|CastToBP_CPlayerState (Game|GetPlayerState PlayerID)))
  (if (> (Utilities|Array|Length _returnvalue) _returnvalue_2)
    (Default|AddCard _asbp_cplayer_state (Utilities|String|StringToName (.CardName (Utilities|Struct|BreakCCardInfo (Utilities|Array|Get(acopy) _returnvalue _returnvalue_2)))))
    (Variables|/Game/Blueprints/PlayerState/BP_CPlayerState.BP_CPlayerState_C|SetPlayerCardCount _asbp_cplayer_state (+ (Variables|/Game/Blueprints/PlayerState/BP_CPlayerState.BP_CPlayerState_C|GetPlayerCardCount _asbp_cplayer_state) 1))
    (Math|Integer|IncrementInt (Utilities|Select :Index PlayerID :Option%200 (Variables|Default|GetPlayer1DeckIndex) :Option%201 (Variables|Default|GetPlayer2DeckIndex)))))

(event Custom|Set%20Game%20Start
  ;[0 0 0] Start Game
  (bind _asbp_cgame_state_base (Utilities|Casting|CastToBP_CGameStateBase (Game|GetGameState)))
  (Default|ReceiveGameStart _asbp_cgame_state_base)
  (bind _asbp_cplayer_state (Utilities|Casting|CastToBP_CPlayerState (Game|GetPlayerState (Variables|/Game/Blueprints/GameState/BP_CGameStateBase.BP_CGameStateBase_C|GetCurrentPlayerTurn _asbp_cgame_state_base))))
  (Default|TurnStart _asbp_cplayer_state)
  (for (_ _array_index) (Variables|Default|GetPlayers)
    (bind _asbp_cplayer_state_2 (Utilities|Casting|CastToBP_CPlayerState (Game|GetPlayerState _array_index)))
    (Default|CurrentPlayerTurn _asbp_cplayer_state_2 (Variables|/Game/Blueprints/GameState/BP_CGameStateBase.BP_CGameStateBase_C|GetCurrentPlayerTurn _asbp_cgame_state_base))))

(event Custom|Set%20Players%20Info
  (params (PlayerID :type Integer))
  ;[0 0 0] Set Player Info
  (bind _asbp_cplayer_state (Utilities|Casting|CastToBP_CPlayerState (Game|GetPlayerState PlayerID)))
  (Variables|/Game/Blueprints/PlayerState/BP_CPlayerState.BP_CPlayerState_C|SetPlayerIndex _asbp_cplayer_state PlayerID)
  (Variables|/Game/Blueprints/PlayerState/BP_CPlayerState.BP_CPlayerState_C|SetWhiteScore _asbp_cplayer_state 0)
  (Variables|/Game/Blueprints/PlayerState/BP_CPlayerState.BP_CPlayerState_C|SetBlackScore _asbp_cplayer_state 0)
  (Variables|/Game/Blueprints/PlayerState/BP_CPlayerState.BP_CPlayerState_C|SetJokerCount _asbp_cplayer_state 3))

(event Custom|Receive%20Player%20Turn%20End
  (params (PlayerID :type Integer))
  ;[0 0 0] Player Turn End
  (bind _asbp_cplayer_state (Utilities|Casting|CastToBP_CPlayerState (Game|GetPlayerState PlayerID)))
  (for _index (range (Variables|/Game/Blueprints/PlayerState/BP_CPlayerState.BP_CPlayerState_C|GetPlayerCardCount _asbp_cplayer_state) 2)
    (CallFunction|AddCardtoDeck PlayerID)
    (bind _asbp_cgame_state_base (Utilities|Casting|CastToBP_CGameStateBase (Game|GetGameState)))
    (Default|CurrentPlayerTurnEnd _asbp_cgame_state_base PlayerID)
    (bind _asbp_cplayer_state_2 (Utilities|Casting|CastToBP_CPlayerState (Game|GetPlayerState (Variables|/Game/Blueprints/GameState/BP_CGameStateBase.BP_CGameStateBase_C|GetCurrentPlayerTurn _asbp_cgame_state_base))))
    (Variables|/Game/Blueprints/PlayerState/BP_CPlayerState.BP_CPlayerState_C|SetCardPlacedCount _asbp_cplayer_state_2 0)
    (Default|TurnStart _asbp_cplayer_state_2)
    (for (_ _array_index) (Variables|Default|GetPlayers)
      (bind _asbp_cplayer_state_3 (Utilities|Casting|CastToBP_CPlayerState (Game|GetPlayerState _array_index)))
      (Default|CurrentPlayerTurn _asbp_cplayer_state_3 (Variables|/Game/Blueprints/GameState/BP_CGameStateBase.BP_CGameStateBase_C|GetCurrentPlayerTurn _asbp_cgame_state_base)))))

(event Custom|Receive%20Player%20Use%20Joker
  (params (PlayerID :type Integer))
  ;[0 0 0] Player Use Joker
  (bind _asbp_cplayer_state (Utilities|Casting|CastToBP_CPlayerState (Game|GetPlayerState PlayerID)))
  (Variables|/Game/Blueprints/PlayerState/BP_CPlayerState.BP_CPlayerState_C|SetJokerCount _asbp_cplayer_state (- (Variables|/Game/Blueprints/PlayerState/BP_CPlayerState.BP_CPlayerState_C|GetJokerCount _asbp_cplayer_state) 1)))

(event EventPostLogin
  (params (NewPlayer :type Player%20Controller%20Object%20Reference))
  ;[0 0 0] Player Log In
  (bind _asbp_cplayer_controller (Utilities|Casting|CastToBP_CPlayerController NewPlayer))
  (Utilities|Array|AddUnique (Variables|Default|GetPlayers) _asbp_cplayer_controller)
  (if (== (Utilities|Array|Length (Variables|Default|GetPlayers)) 2)
    (Utilities|FlowControl|Delay 5.0)
    (for _index (range 0 (- (Utilities|Array|Length (Variables|Default|GetPlayers)) 1))
      (CallFunction|SetPlayersInfo _index)
      (for _index_2 (range 0 2)
        (CallFunction|AddCardtoDeck _index)))
    (CallFunction|SetGameStart)))

(fn ConstructionScript)