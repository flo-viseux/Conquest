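; BP_CPlayerPawn is a player pawn, apparently for a card game, that positions itself at a fixed elevated spot on BeginPlay.
; Pressing P requests a game start, running the start logic directly with authority or going through a server event from remote clients.
; That logic casts the game mode to BP_CGameModeBase and calls SetGameStart.
; Disconnected leftover nodes cover adding hand cards and placing card actors on the board.
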(event Custom|Request%20Server%20Game%20Start
  (Networking|SwitchHasAuthority
    (:Authority
      (bind _asbp_cgame_mode_base (Utilities|Casting|CastToBP_CGameModeBase (Game|GetGameMode)))
      (Default|SetGameStart _asbp_cgame_mode_base))
    (:Remote
      (CallFunction|SRV-StartGame))))

(event Custom|SRV%20-%20Start%20game
  (bind _asbp_cgame_mode_base (Utilities|Casting|CastToBP_CGameModeBase (Game|GetGameMode)))
  (Default|SetGameStart _asbp_cgame_mode_base))

(event EventBeginPlay
  (Transformation|SetActorLocationAndRotation "0.000000,400.000000,600.000000" "0.000000,-90.000000,0.000000"))

(event Input|KeyboardEvents|P
  (params (Key :type Key%20Structure :default "None"))
  (:Pressed
    (CallFunction|RequestServerGameStart)))

(fn ConstructionScript)