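; Player controller for a turn-based card board game, handling the HUD, hand, turn input and score updates.
; Dragging a selected card moves a preview actor over the cell under the mouse; releasing requests placement.
; Placement, turn end and Joker use reach the game mode directly on authority or through server RPCs, with a hard-coded position offset on the authority side.
; Input is enabled only during the player's turn.
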(event Custom|SRV%20-%20Request%20Play%20Card
  (params (CellPos :type Vector) (PlayerId :type Integer) (CardName :type Name))
  ;[0 0 0] Play Card
  (bind _asbp_cgame_mode_base (Utilities|Casting|CastToBP_CGameModeBase (Game|GetGameMode)))
  (Default|PlaceCardonBoard _asbp_cgame_mode_base CellPos CardName PlayerId))

(event Custom|Add%20Card
  (params (CardDataRowName :type Name))
  ;[0 0 0] Add Card To Hand
  (bind _returnvalue (Utilities|GetDataTableRow "/Game/Blueprints/Cards/DT_CCardInfo.DT_CCardInfo" CardDataRowName)
    (:then
      (Utilities|Array|AddUnique (Variables|Default|GetCurrentCardsHand) (Utilities|Struct|MakeCCardInfo (.cardname _returnvalue) (.cardtype _returnvalue) (Variables|Default|GetIndex) (.texture1 _returnvalue) (.texture2 _returnvalue) (.links _returnvalue)))
      (Utilities|IsValid (Variables|Default|GetW_PlayerHand)
        (:Is%20Valid
          (Default|AddCardtoHand (Variables|Default|GetW_PlayerHand) (Utilities|Struct|MakeCCardInfo (.cardname _returnvalue) (.cardtype _returnvalue) (Variables|Default|GetIndex) (.texture1 _returnvalue) (.texture2 _returnvalue) (.links _returnvalue))))))))

(event Custom|Receive%20Turn%20End
  (bind _w_playerhud (Variables|Default|GetW_PlayerHUD))
  ;[0 0 0] Turn End
  (Input|DisableInput self)
  (Utilities|IsValid _w_playerhud
    (:Is%20Valid
      (Default|SetEnableEndButton _w_playerhud false)
      (Default|SetEnableJokerButton _w_playerhud false)
      (Networking|SwitchHasAuthority
        (:Authority
          (bind _asbp_cgame_mode_base (Utilities|Casting|CastToBP_CGameModeBase (Game|GetGameMode)))
          (Default|ReceivePlayerTurnEnd _asbp_cgame_mode_base (Variables|Default|GetIndex)))
        (:Remote
          (CallFunction|SRV-SENDPlayerTurnEnd (Variables|Default|GetIndex)))))))

(event Custom|Receive%20Current%20Player%20Turn
  (params (CurrentTurnPlayerID :type Integer))
  ;[0 0 0] Current Player Turn
  (Default|UpdateTurn (Variables|Default|GetW_PlayerHUD) CurrentTurnPlayerID))

(event Custom|Receive%20Update%20Current%20Joker%20Remains
  (params (CurrentJokerRemains :type Integer))
  ;[0 0 0] Current Joker Remains
  (Variables|Default|SetCurrentJokerRemains CurrentJokerRemains)
  (Default|UpdateCurrentJokerRemains (Variables|Default|GetW_PlayerHUD) CurrentJokerRemains))

(event Custom|SRV%20-%20Send%20Use%20Joker
  (params (PlayerID :type Integer))
  ;[0 0 0] Use Joker
  (bind _asbp_cgame_mode_base (Utilities|Casting|CastToBP_CGameModeBase (Game|GetGameMode)))
  (Default|ReceivePlayerUseJoker _asbp_cgame_mode_base PlayerID))

(event Custom|Use%20Joker
  ;[0 0 0] Use Joker
  (Networking|SwitchHasAuthority
    (:Authority
      (bind _asbp_cgame_mode_base (Utilities|Casting|CastToBP_CGameModeBase (Game|GetGameMode)))
      (Default|ReceivePlayerUseJoker _asbp_cgame_mode_base (Variables|Default|GetIndex)))
    (:Remote
      (CallFunction|SRV-SendUseJoker (Variables|Default|GetIndex)))))

(event Custom|TurnStart
  (bind _w_playerhud (Variables|Default|GetW_PlayerHUD))
  ;[0 0 0] Turn Start
  (Input|EnableInput self)
  (Utilities|IsValid _w_playerhud
    (:Is%20Valid
      (Default|SetEnableEndButton _w_playerhud true)
      (if (> (Variables|Default|GetCurrentJokerRemains) 0)
        (Default|SetEnableJokerButton _w_playerhud true)))))

(event Custom|Receive%20Player%20Info
  (params (PlayerID :type Integer))
  ;[0 0 0] Player Info
  (bind _output_get (Variables|Default|SetIndex PlayerID))
  (Default|SetPlayerInfo (Variables|Default|GetW_PlayerHUD) _output_get))

(event Custom|SRV%20-%20Send%20Player%20Turn%20End
  (params (PlayerID :type Integer))
  ;[0 0 0] Turn End
  (bind _asbp_cgame_mode_base (Utilities|Casting|CastToBP_CGameModeBase (Game|GetGameMode)))
  (Default|ReceivePlayerTurnEnd _asbp_cgame_mode_base PlayerID))

(event Custom|Remove%20Card
  (params (Card%20Data%20Row%20Name :type Name))
  ;[0 0 0] Remove Card From Hand
  (bind _returnvalue (Utilities|GetDataTableRow "/Game/Blueprints/Cards/DT_CCardInfo.DT_CCardInfo" Card%20Data%20Row%20Name)
    (:then
      (Utilities|Array|RemoveItem (Variables|Default|GetCurrentCardsHand) (Utilities|Struct|MakeCCardInfo (.cardname _returnvalue) (.cardtype _returnvalue) (Variables|Default|GetIndex) (.texture1 _returnvalue) (.texture2 _returnvalue) (.links _returnvalue)))
      (Utilities|IsValid (Variables|Default|GetW_PlayerHand)
        (:Is%20Valid
          (Default|RemoveCardfromHnad (Variables|Default|GetW_PlayerHand) (Utilities|Struct|MakeCCardInfo (.cardname _returnvalue) (.cardtype _returnvalue) (Variables|Default|GetIndex) (.texture1 _returnvalue) (.texture2 _returnvalue) (.links _returnvalue))))))))

(event Custom|UpdateBlackScore
  (params (NewBlackScore :type Integer))
  ;[0 0 0] Update Scores
  (Default|UpdateBlackScore (Variables|Default|GetW_PlayerHUD) NewBlackScore))

(event Custom|UpdateWhiteScore
  (params (NewWhiteScore :type Integer))
  ;[0 0 0] Update Scores
  (Default|UpdateWhiteScore (Variables|Default|GetW_PlayerHUD) NewWhiteScore))

(event Input|EnhancedActionEvents|EnhancedInputActionIA_Click
  (params (ActionValue :type Boolean) (ElapsedSeconds :type Float%20%28double-precision%29) (TriggeredSeconds :type Float%20%28double-precision%29) (InputAction :type Input%20Action%20Object%20Reference :default "/Game/Blueprints/Player/Inputs/IA_Click.IA_Click"))
  (bind _w_playerhand (Variables|Default|GetW_PlayerHand))
  (bind _currentselectedcard (Variables|/Game/Blueprints/Player/W_PlayerHand.W_PlayerHand_C|GetCurrentSelectedCard _w_playerhand))
  (:Triggered
    ;[0 0 0] Drag Card only on cells
    (if (!= _currentselectedcard "")
      (Default|SetCCardInfo (Variables|Default|GetCardActor) (Variables|Default|GetIndex) _currentselectedcard)
      (bind _returnvalue (Class|CPlayerController|GetCellUnderMouse))
      (bind _asbp_ccell_actor (Utilities|Casting|CastToBP_CCellActor _returnvalue)
        (:then
          (Widget|SetVisibility (Variables|Default|GetW_PlayerHand) "Hidden")
          (Networking|SwitchHasAuthority
            (:Authority
              (Transformation|SetActorLocation (Variables|Default|GetCardActor) (- (Variables|/Game/Blueprints/Grid/BP_CCellActor.BP_CCellActor_C|GetCellPos _asbp_ccell_actor) "650.000000,450.000000,-1.000000") false false))
            (:Remote
              (Transformation|SetActorLocation (Variables|Default|GetCardActor) (+ (Variables|/Game/Blueprints/Grid/BP_CCellActor.BP_CCellActor_C|GetCellPos _asbp_ccell_actor) "0.000000,0.000000,1.000000") false false))))
        (:CastFailed
          (Widget|SetVisibility (Variables|Default|GetW_PlayerHand) "Visible")
          (Transformation|SetActorLocation (Variables|Default|GetCardActor) "10000.000000,10000.000000,10000.000000" false false)))))
  (:Completed
    ;[0 0 0] Play Card
    (Widget|SetVisibility (Variables|Default|GetW_PlayerHand) "Visible")
    (Transformation|SetActorLocation (Variables|Default|GetCardActor) "100000.000000,10000.000000,100000.000000" false false)
    (if (!= (Variables|/Game/Blueprints/Player/W_PlayerHand.W_PlayerHand_C|GetCurrentSelectedCard (Variables|Default|GetW_PlayerHand)) "")
      (bind _returnvalue_2 (Class|CPlayerController|GetCellUnderMouse))
      (bind _asbp_ccell_actor_2 (Utilities|Casting|CastToBP_CCellActor _returnvalue_2))
      (Networking|SwitchHasAuthority
        (:Authority
          (bind _asbp_cgame_mode_base (Utilities|Casting|CastToBP_CGameModeBase (Game|GetGameMode)))
          (Default|PlaceCardonBoard _asbp_cgame_mode_base (- (Variables|/Game/Blueprints/Grid/BP_CCellActor.BP_CCellActor_C|GetCellPos _asbp_ccell_actor_2) "650.000000,450.000000,0.000000") (Variables|/Game/Blueprints/Player/W_PlayerHand.W_PlayerHand_C|GetCurrentSelectedCard (Variables|Default|GetW_PlayerHand)) (Variables|Default|GetIndex)))
        (:Remote
          (CallFunction|SRV-RequestPlayCard (Variables|/Game/Blueprints/Grid/BP_CCellActor.BP_CCellActor_C|GetCellPos _asbp_ccell_actor_2) (Variables|Default|GetIndex) (Variables|/Game/Blueprints/Player/W_PlayerHand.W_PlayerHand_C|GetCurrentSelectedCard (Variables|Default|GetW_PlayerHand))))))))

(event EventBeginPlay
  (bind _returnvalue (PlayerController|LocalPlayerSubsystems|GetEnhancedInputLocalPlayerSubsystem))
  ;[0 0 0] BeginPlay
  (Input|DisableInput self)
  (Utilities|IsValid _returnvalue
    (:Is%20Valid
      (Input|AddMappingContext _returnvalue "/Game/Blueprints/Player/Inputs/IMC_Conquest.IMC_Conquest" 0 "(bIgnoreAllPressedKeysUntilRelease=True,bForceImmediately=False,bNotifyUserSettings=False)")
      (bind _returnvalue_2 (UserInterface|CreateWidget "/Game/Blueprints/Player/W_PlayerHUD.W_PlayerHUD_C" self))
      (bind _output_get (Variables|Default|SetW_PlayerHUD _returnvalue_2))
      (UserInterface|Viewport|AddtoViewport _output_get 0)
      (Variables|Default|SetW_PlayerHand (Variables|/Game/Blueprints/Player/W_PlayerHUD.W_PlayerHUD_C|GetW_PlayerHand _output_get))
      (bind _returnvalue_3 (Game|SpawnActorfromClass "/Game/Blueprints/Cards/BP_CCardActorPreview.BP_CCardActorPreview_C" (Math|Transform|MakeTransform "100000.000000,1000000.000000,1000000.000000") "AlwaysSpawn" "MultiplyWithRoot" 0 0))
      (Variables|Default|SetCardActor _returnvalue_3))))

(fn ConstructionScript)

(fn OnRepWPlayerHand)